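; BP_ClockStarter is a trigger actor that starts the clock sequence once Lady Maria is gone from the level.
; When a BloodBornCharacter overlaps StartRange and no BP_LadyMaria3 actors exist, a DoOnce lets the sequence run a single time.
; It plays a 2D sound, waits briefly, then enables rotation on the first BP_ClockActor found and calls its MoveTickTok.
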(event `self.StartRange.OnComponentBeginOverlap`
  (params (OverlappedComponent :type "PrimitiveComponent Object Reference") (OtherActor :type "Actor Object Reference") (OtherComp :type "PrimitiveComponent Object Reference") (OtherBodyIndex :type Integer) (bFromSweep :type Boolean) (SweepResult :type "HitResult Structure (by ref)"))
  (cast `BloodBornCharacter` OtherActor)
  (bind _outactors (`GameplayStatics.GetAllActorsOfClass` "/Game/Enemy/Boss_LadyMaria/BP_LadyMaria3.BP_LadyMaria3_C"))
  (if (== (`KismetArrayLibrary.Array_Length` _outactors) 0)
    (`/Engine/EditorBlueprintResources/StandardMacros.DoOnce` false
      (:`Completed`
        (bind _outactors_2 (`GameplayStatics.GetAllActorsOfClass` "/Game/Choi/BP_ClockActor.BP_ClockActor_C"))
        (`GameplayStatics.PlaySound2D` "/Game/Enemy/SoundEffect/videoplayback__cut_23sec_.videoplayback__cut_23sec_" 1.0 1.0 0.0 null null)
        (`KismetSystemLibrary.Delay` 2.5)
        (bind _output (`|GetArrayItem` _outactors_2))
        (set `ClockActor.bIsRotateStart` true _output)
        (`ClockActor.MoveTickTok` _output)))))

(fn `UserConstructionScript`)