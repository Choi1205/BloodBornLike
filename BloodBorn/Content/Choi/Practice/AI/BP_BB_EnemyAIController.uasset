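; AI controller for a stay-type enemy that runs a behavior tree and caches its possessed BP_StayEnemy on BeginPlay.
; PawnSensing sightings of the third-person player write CanSeePlayer and PlayerTarget to the Blackboard.
; A retriggerable delay of twice the sensing interval acts as a lose-sight timeout, clearing CanSeePlayer and immediately stopping the enemy's attack montage.
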(event `self.ReceiveBeginPlay`
  (`self.RunBehaviorTree` (`self.AIBehaviorTree`))
  (bind _asbp_stay_enemy (cast `/Game/Choi/Practice/BP_StayEnemy` (`self.K2_GetPawn`)))
  (set `self.EnemyREF` _asbp_stay_enemy))

(event `self.PawnSensing.OnSeePawn`
  (params (Pawn :type "Pawn Object Reference"))
  (bind _asbp_third_person_character (cast `/Game/ThirdPerson/Blueprints/BP_ThirdPersonCharacter` Pawn))
  (`self.SetCanSeePlayer` true _asbp_third_person_character)
  (`KismetSystemLibrary.RetriggerableDelay` (* (`PawnSensingComponent.SensingInterval` (`self.PawnSensing`)) 2.0))
  (`self.SetCanSeePlayer` false)
  (`AnimInstance.Montage_Stop` (`SkeletalMeshComponent.GetAnimInstance` (`Character.Mesh` (`self.EnemyREF`))) 0.0 "/Game/Choi/Practice/EnemyModel/Melee/EnemyAttack.EnemyAttack"))

(fn `SetCanSeePlayer`
  (params (CanSeePlayer :type Boolean) (PlayerObject :type "Object Object Reference"))
  (bind _returnvalue (`AIBlueprintHelperLibrary.GetBlackboard` self))
  (if CanSeePlayer
    (`BlackboardComponent.SetValueAsBool` _returnvalue "CanSeePlayer" true)
    (`BlackboardComponent.SetValueAsObject` _returnvalue "PlayerTarget" PlayerObject)
    (else
      (`BlackboardComponent.SetValueAsBool` _returnvalue "CanSeePlayer" false))))

(fn `UserConstructionScript`)