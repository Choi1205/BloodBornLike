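; BP_StayEnemy is a practice melee enemy that, as wired, only prints a debug message when its damage collision overlaps the third-person character while CanDealDamage is set.
; BeginPlay calls Randompatrol, but that event and the detection, seek and attack events are empty.
; Disconnected chains hold the intended AI: random patrol, timer-driven AIMoveTo pursuit, and a montage attack facing the player.
; TowardPlayer's direction calculation is also left unconnected.
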(event `self.ReceiveBeginPlay`
  (`self.Randompatrol`))

(event `Randompatrol`)

(event `MoveToPlayer`)

(event `self.PlayerCollisionDetection.OnComponentBeginOverlap`
  (params (OverlappedComponent :type "PrimitiveComponent Object Reference") (OtherActor :type "Actor Object Reference") (OtherComp :type "PrimitiveComponent Object Reference") (OtherBodyIndex :type Integer) (bFromSweep :type Boolean) (SweepResult :type "HitResult Structure (by ref)")))

(event `self.PlayerCollisionDetection.OnComponentEndOverlap`
  (params (OverlappedComponent :type "PrimitiveComponent Object Reference") (OtherActor :type "Actor Object Reference") (OtherComp :type "PrimitiveComponent Object Reference") (OtherBodyIndex :type Integer)))

(event `SeekPlayer`)

(event `StopSeekPlayer`)

(event `self.PlayerAttackCollisionDetection.OnComponentBeginOverlap`
  (params (OverlappedComponent :type "PrimitiveComponent Object Reference") (OtherActor :type "Actor Object Reference") (OtherComp :type "PrimitiveComponent Object Reference") (OtherBodyIndex :type Integer) (bFromSweep :type Boolean) (SweepResult :type "HitResult Structure (by ref)")))

(event `self.PlayerAttackCollisionDetection.OnComponentEndOverlap`
  (params (OverlappedComponent :type "PrimitiveComponent Object Reference") (OtherActor :type "Actor Object Reference") (OtherComp :type "PrimitiveComponent Object Reference") (OtherBodyIndex :type Integer)))

(event `self.DamageCollision.OnComponentBeginOverlap`
  (params (OverlappedComponent :type "PrimitiveComponent Object Reference") (OtherActor :type "Actor Object Reference") (OtherComp :type "PrimitiveComponent Object Reference") (OtherBodyIndex :type Integer) (bFromSweep :type Boolean) (SweepResult :type "HitResult Structure (by ref)"))
  (cast `/Game/ThirdPerson/Blueprints/BP_ThirdPersonCharacter` OtherActor)
  (if (`self.CanDealDamage`)
    (`KismetSystemLibrary.PrintString` "PlayerDamaged")))

(fn `UserConstructionScript`)