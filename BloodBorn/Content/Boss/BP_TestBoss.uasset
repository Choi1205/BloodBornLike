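; BP_TestBoss is a test boss that tracks its health and displays it on a WB_BossHUD widget.
; On BeginPlay it creates the HUD, adds it to the viewport and fills health to maximum.
; AnyDamage subtracts clamped damage and passes it with current and max health to the HUD's AllDamageSystem.
; Death below 1 HP only prints a string, and the boss's own UpdateHealthUI function is an empty stub.
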(event `self.ReceiveBeginPlay`
  ;[1 1 1] 화면에 프로그래스 바 UI창 띄우기
  (bind _returnvalue (`|CreateWidget` "/Game/UI/WB_BossHUD.WB_BossHUD_C"))
  (bind _output_get (set `self.HUD_Main` _returnvalue))
  (`UserWidget.AddToViewport` _output_get 0)
  ;[1 1 1] 게임 시작 시 HP가 꽉 채워진 상태로 시작
  (bind _output_get_2 (set `self.CurrentHP` (`self.MaxHP`)))
  (`/Game/UI/WB_BossHUD.UpdateHealthUI` (`self.HUD_Main`) _output_get_2 (`self.MaxHP`)))

(event `self.ReceiveAnyDamage`
  (params (Damage :type "Float (single-precision)") (DamageType :type "DamageType Object Reference") (InstigatedBy :type "Controller Object Reference") (DamageCauser :type "Actor Object Reference"))
  ;[1 1 1] 데미지를 입으면 HP가 떨어진다.
  (bind _output_get (set `self.CurrentHP` (`KismetMathLibrary.FClamp` (- (`self.CurrentHP`) Damage) 0.0 (`self.MaxHP`))))
  (`/Game/UI/WB_BossHUD.All_DamageSystem` (`self.HUD_Main`) Damage _output_get (`self.MaxHP`))
  (if (< (`self.CurrentHP`) 1.0)
    ;[1 1 1] HP가 1보다 작으면 죽는다.
    (if (< (`self.CurrentHP`) 1.0)
      (`KismetSystemLibrary.PrintString` "Death"))))

(fn `UpdateHealthUI`
  (params (CurrentHP :type "Float (double-precision)") (MaxHP :type "Float (double-precision)")))

(fn `UserConstructionScript`)