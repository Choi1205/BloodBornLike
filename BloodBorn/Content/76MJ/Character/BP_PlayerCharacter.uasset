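; Player character Blueprint with a lock-on toggle on IA_Lockon, though its engage and disengage events are empty.
; Disconnected graphs hold the lock-on logic: sphere-trace for BPI_Lockon actors, pick the nearest, steer control rotation toward it and switch movement orientation.
; A looping timer there would call BreakLockOn, which disengages beyond a set distance.
; Attack montage and parry-hit fragments are also unwired, leaving attack and fire inputs empty.
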(event `EnhancedInput|/Game/ThirdPerson/Input/Actions/IA_NormalAttack`
  (params (ActionValue :type Boolean) (ElapsedSeconds :type "Float (double-precision)") (TriggeredSeconds :type "Float (double-precision)") (InputAction :type "InputAction Object Reference" :default "/Game/ThirdPerson/Input/Actions/IA_NormalAttack.IA_NormalAttack")))

(event `Engage Lock`)

(event `EnhancedInput|/Game/ThirdPerson/Input/Actions/IA_GunFire`
  (params (ActionValue :type Boolean) (ElapsedSeconds :type "Float (double-precision)") (TriggeredSeconds :type "Float (double-precision)") (InputAction :type "InputAction Object Reference" :default "/Game/ThirdPerson/Input/Actions/IA_GunFire.IA_GunFire")))

(event `self.ReceiveTick`
  (params (DeltaSeconds :type "Float (single-precision)")))

(event `Disengage Lockon`)

(event `EnhancedInput|/Game/ThirdPerson/Input/Actions/IA_Lockon`
  (params (ActionValue :type Boolean) (ElapsedSeconds :type "Float (double-precision)") (TriggeredSeconds :type "Float (double-precision)") (InputAction :type "InputAction Object Reference" :default "/Game/ThirdPerson/Input/Actions/IA_Lockon.IA_Lockon"))
  (:`Started`
    (if (`self.LockonEngaged?`)
      (`self.Disengage Lockon`)
      (else
        (`self.Engage Lock`)))))

(fn `BreakLockOn`
  (`self.TargetActor`
    (:`then`
      (if (>= (`KismetMathLibrary.Vector_Distance` (`self.K2_GetActorLocation`) (`self.K2_GetActorLocation` (`self.TargetActor`))) 3000.0)
        (`self.Disengage Lockon`)))
    (:`else`)))

(fn `UserConstructionScript`)