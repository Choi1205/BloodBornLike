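; BP_LadyMaria3 is a Lady Maria boss Blueprint that drives the boss HUD from its health.
; On BeginPlay it creates WB_BossHUD, adds it to the viewport and initializes the health display.
; Tick polls HealthPoint against a cached BeforeHealth, passing any difference to the HUD's AllDamageSystem as damage, along with current and max health.
; EndPlay hides the HUD rather than removing it.
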(event `self.ReceiveBeginPlay`
  (bind _healthpoint (`self.healthPoint`))
  (bind _returnvalue (`|CreateWidget` "/Game/UI/WB_BossHUD.WB_BossHUD_C"))
  (bind _output_get (set `self.HUD_Main` _returnvalue))
  (`UserWidget.AddToViewport` _output_get 0)
  (`/Game/UI/WB_BossHUD.UpdateHealthUI` (`self.HUD_Main`) _healthpoint (`self.maxHealthPoint`))
  (set `self.beforeHealth` _healthpoint))

(event `self.ReceiveTick`
  (params (DeltaSeconds :type "Float (single-precision)"))
  (bind _beforehealth (`self.beforeHealth`))
  (bind _healthpoint (`self.healthPoint`))
  (if (not (== _beforehealth _healthpoint))
    (`/Game/UI/WB_BossHUD.All_DamageSystem` (`self.HUD_Main`) (- _beforehealth _healthpoint) _healthpoint (`self.maxHealthPoint`))
    (set `self.beforeHealth` (`self.healthPoint`))))

(event `self.ReceiveEndPlay`
  (params (EndPlayReason :type "EEndPlayReason Enum" :default "Destroyed"))
  (`Widget.SetVisibility` (`self.HUD_Main`) "Hidden"))

(fn `UserConstructionScript`)