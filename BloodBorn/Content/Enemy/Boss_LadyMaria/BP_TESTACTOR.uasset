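; A test actor in the Lady Maria boss folder that repeatedly restarts four pairs of Niagara effects.
; Tick advances four independent timers, each of which resets and reactivates its pair on passing a threshold, with two pairs on a slower interval and two on a faster one.
; An upward movement step driven by Upspeed is present but disconnected, so the actor's graph never moves it.
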(event `self.ReceiveTick`
  (params (DeltaSeconds :type "Float (single-precision)"))
  (set `self.timer1` (+ (`self.timer1`) DeltaSeconds))
  (set `self.timer2` (+ (`self.timer2`) DeltaSeconds))
  (set `self.timer3` (+ (`self.timer3`) DeltaSeconds))
  (set `self.timer4` (+ (`self.timer4`) DeltaSeconds))
  (`|ExecutionSequence`
    (:`then_0`
      (if (> (`self.timer1`) 0.4)
        (set `self.timer1` 0.0)
        (`ActorComponent.Activate` (`self.Niagara1-1`) true)
        (`ActorComponent.Activate` (`self.Niagara1-2`) true)))
    (:`then_1`
      (if (> (`self.timer2`) 0.1)
        (set `self.timer2` 0.0)
        (`ActorComponent.Activate` (`self.Niagara2-2`) true)
        (`ActorComponent.Activate` (`self.Niagara2-1`) true)))
    (:`then_2`
      (if (> (`self.timer3`) 0.4)
        (set `self.timer3` 0.0)
        (`ActorComponent.Activate` (`self.Niagara3-1`) true)
        (`ActorComponent.Activate` (`self.Niagara3-2`) true)))
    (:`then_3`
      (if (> (`self.timer4`) 0.1)
        (set `self.timer4` 0.0)
        (`ActorComponent.Activate` (`self.Niagara4-1`) true)
        (`ActorComponent.Activate` (`self.Niagara4-2`) true)))))

(fn `UserConstructionScript`)